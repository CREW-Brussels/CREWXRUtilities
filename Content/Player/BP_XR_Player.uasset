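; XR player Blueprint that feeds hand tracking and auto-scales the body mesh to the player's height.
; When locally controlled, Tick sends both hands' tracking, height and horizontal speed through UpdateHandState for replication.
; ProcessTracking remaps joint rotations per hand, but its tracking source is disabled since ViveOpenXR's removal.
; Auto height follows rising camera height instantly and falling height slowly, driving mesh scale, offset and floor height.
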(event Custom|Update%20Hand%20State
  (params (HandState :type S%20Tr%20XR%20Hand%20State%20Structure))
  ;[1 1 1] Replicate Hand Tracking
  (Variables|Default|SetHandState HandState))

(event EventBeginPlay
  ;[1 1 1] Init
  (Variables|Default|SetLocation (* (Transformation|GetWorldLocation (Variables|Default|GetParentRelativeAttachment)) "1.000000,1.000000,0.000000")))

(event EventTick
  (params (DeltaSeconds :type Float%20%28single-precision%29))
  (bind _mesh (Variables|Character|GetMesh))
  (bind _vrreplicatedcamera (Variables|Default|GetVRReplicatedCamera))
  (bind _parentrelativeattachment (Variables|Default|GetParentRelativeAttachment))
  (bind _returnvalue (Transformation|GetWorldLocation _parentrelativeattachment))
  (bind _returnvalue_2 (Transformation|GetWorldRotation _vrreplicatedcamera))
  (bind _returnvalue_3 (Transformation|GetWorldLocation _vrreplicatedcamera))
  (bind _returnvalue_4 (Math|Vector|GetForwardVector _returnvalue_2))
  (bind _returnvalue_5 (* _returnvalue "1.000000,1.000000,0.000000"))
  (bind _returnvalue_6 (* _returnvalue_4 -1e+01))
  (bind _returnvalue_7 (+ _returnvalue_3 _returnvalue_6))
  ;[1 1 1] Hand Tracking
  (Utilities|FlowControl|Sequence
    (:then_0
      (if (Pawn|IsLocallyControlled)
        ;;[0.15 0 0 0.5] TODO: These were disabled after removing ViveOpenXR
        (bind (_tracked _rotations _location) (CallFunction|ProcessTracking false 0 0 false))
        (bind (_tracked_2 _rotations_2 _location_2) (CallFunction|ProcessTracking true 0 0 false))
        (CallFunction|UpdateHandState (Utilities|Struct|MakeSTr_XRHandState _tracked _tracked_2 _rotations _rotations_2 _location _location_2 (+ (- 165.0 (.Z (Math|Vector|BreakVector _returnvalue))) (Variables|Default|GetFloorHeight)) (/ (Math|Vector|VectorLength (- _returnvalue_5 (Variables|Default|GetLocation))) DeltaSeconds)))
        (Variables|Default|SetLocation _returnvalue_5)))
    (:then_1
      ;[1 1 1] Auto Height
      (if (> (.z _returnvalue_7) (Variables|Default|GetMeanHeight))
        (Variables|Default|SetMeanHeight (.z _returnvalue_7))
        (else
          (bind _output_get (Variables|Default|SetMeanHeight (Math|Float|Lerp (Variables|Default|GetMeanHeight) (.z _returnvalue_7) 0.005)))))
      (Transformation|SetRelativeScale3D _mesh (Math|Conversions|ToVector(Float) (/ _output_get 1.7e+02)))
      (Transformation|SetRelativeLocation _mesh (Math|Vector|MakeVector -5.0 0.0 (* _output_get -1.0)) false true)
      (Variables|Default|SetFloorHeight (- _output_get 1.7e+02)))))

(fn ConstructionScript)

(fn ProcessTracking
  (params (Handedness :type Boolean) (HandKeyPositions :type Array%20of%20Vectors) (HandKeyRotations :type Array%20of%20Quat%20Structures) (isValid :type Boolean))
  (Utilities|FlowControl|Sequence
    (:then_0
      (if isValid
        (for _array_element HandKeyRotations
          (if Handedness
            (Utilities|Array|Add (LocalVariables|GetRotations_Temp) (Math|Rotator|MakeRotator (+ (* (.Roll (Math|Rotator|BreakRotator (Class|KismetMathLibrary|QuatRotator _array_element))) -1.0) 9e+01) (* (.Pitch (Math|Rotator|BreakRotator (Class|KismetMathLibrary|QuatRotator _array_element))) -1.0) (+ (.Yaw (Math|Rotator|BreakRotator (Class|KismetMathLibrary|QuatRotator _array_element))) 1.8e+02)))
            (else
              (Utilities|Array|Add (LocalVariables|GetRotations_Temp) (Math|Rotator|MakeRotator (+ (* (.Roll (Math|Rotator|BreakRotator (Class|KismetMathLibrary|QuatRotator _array_element))) 1.0) 9e+01) (+ (* (.Pitch (Math|Rotator|BreakRotator (Class|KismetMathLibrary|QuatRotator _array_element))) -1.0) 1.8e+02) (+ (.Yaw (Math|Rotator|BreakRotator (Class|KismetMathLibrary|QuatRotator _array_element))) 1.8e+02))))))
        (LocalVariables|SetLocation_Temp (Utilities|Array|Get(acopy) HandKeyPositions 1))))
    (:then_1
      (return isValid (LocalVariables|GetRotations_Temp) (LocalVariables|GetLocation_Temp)))))